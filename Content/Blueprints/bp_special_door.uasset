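; A special door Blueprint that the player toggles with the E key through the Doorrotation timeline.
; E plays or reverses the timeline based on Doorclosed, which Tick derives from the Door track value.
; Timeline updates set DoorBody to a fixed relative offset and yaw, as the track-driven rotator is unused.
; Both Box begin and end overlap enable input for player 0, so input is never disabled.
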(event OnComponentBeginOverlap(Box)
  (params (OverlappedComponent :type Primitive%20Component%20Object%20Reference) (OtherActor :type Actor%20Object%20Reference) (OtherComp :type Primitive%20Component%20Object%20Reference) (OtherBodyIndex :type Integer) (bFromSweep :type Boolean) (SweepResult :type Hit%20Result%20Structure%20%28by%20ref%29))
  (Input|EnableInput (Game|GetPlayerController 0)))

(event OnComponentEndOverlap(Box)
  (params (OverlappedComponent :type Primitive%20Component%20Object%20Reference) (OtherActor :type Actor%20Object%20Reference) (OtherComp :type Primitive%20Component%20Object%20Reference) (OtherBodyIndex :type Integer))
  (Input|EnableInput (Game|GetPlayerController 0)))

(event EventTick
  (params (DeltaSeconds :type Float%20%28single-precision%29))
  (Variables|Default|Setdoorclosed (< (stale Input|KeyboardEvents|E _door) 1.0)))

(event Input|KeyboardEvents|E
  (params (Key :type Key%20Structure :default "None"))
  (:Pressed
    (if (Variables|Default|Getdoorclosed)
      (bind _door (Timeline|doorrotation Play)
        (:Update
          (Transformation|SetRelativeLocationAndRotation (Variables|Default|GetDoor%20Body) "0.000000,-60.000000,0.000000" "0.000000,105.000000,0.000000" false false)))
      (else
        (Timeline|doorrotation Reverse)))))

(fn ConstructionScript)
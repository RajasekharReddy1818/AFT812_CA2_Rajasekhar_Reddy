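; Keypad door Blueprint that swings open once enough items have been collected.
; A collect event increments the collected count, and a check event compares it to the maximum, opening the door through a DoOnce so it fires only once.
; Opening plays a timeline that lerps the door body's yaw from closed to an open angle.
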(event Custom|open%20door
  (bind _door_rotation (Timeline|opendoor%20anim Play)
    (:Update
      (Transformation|SetRelativeRotation (Variables|Default|GetDoor%20Body) (Math|Rotator|MakeRotator 0.0 0.0 (Math|Float|Lerp 0.0 8e+01 _door_rotation)) false false))))

(event Custom|collect%20items
  (Math|Integer|IncrementInt (Variables|Default|Getcurrentitemscollected)))

(event Custom|open%20door%20check
  (if (>= (Variables|Default|Getcurrentitemscollected) (Variables|Default|Getmaxitemscollected))
    (Utilities|FlowControl|DoOnce false
      (:Completed
        (CallFunction|OpenDoor)))))

(fn ConstructionScript)
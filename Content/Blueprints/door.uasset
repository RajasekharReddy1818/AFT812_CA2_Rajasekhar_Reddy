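; Door actor that the player operates with the E key, enabled when something overlaps its Box.
; E plays or reverses the NewDoorRotation timeline, based on a closed flag refreshed each Tick from its Door track.
; Timeline updates set DoorBody to a fixed rotation, leaving the track-driven rotator unused.
; End overlap also calls EnableInput, so input is never disabled.
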(event OnComponentBeginOverlap(Box)
  (params (OverlappedComponent :type Primitive%20Component%20Object%20Reference) (OtherActor :type Actor%20Object%20Reference) (OtherComp :type Primitive%20Component%20Object%20Reference) (OtherBodyIndex :type Integer) (bFromSweep :type Boolean) (SweepResult :type Hit%20Result%20Structure%20%28by%20ref%29))
  (Input|EnableInput (Game|GetPlayerController 0)))

(event OnComponentEndOverlap(Box)
  (params (OverlappedComponent :type Primitive%20Component%20Object%20Reference) (OtherActor :type Actor%20Object%20Reference) (OtherComp :type Primitive%20Component%20Object%20Reference) (OtherBodyIndex :type Integer))
  (Input|EnableInput (Game|GetPlayerController 0)))

(event EventTick
  (params (DeltaSeconds :type Float%20%28single-precision%29))
  (Variables|Default|Setdoorclosed (< (stale Input|KeyboardEvents|E _door) 1.0)))

(event Input|KeyboardEvents|E
  (params (Key :type Key%20Structure :default "None"))
  (:Pressed
    (if (Variables|Default|Getdoorclosed)
      (bind _door (Timeline|new%20door%20rotation Play)
        (:Update
          (Transformation|SetRelativeRotation (Variables|Default|GetDoor%20Body) "0.000000,80.000000,0.000000" false false)))
      (else
        (Timeline|new%20door%20rotation Reverse)))))

(fn ConstructionScript)